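; Anim notify that plays a foley sound at the mesh's location for a gameplay-tag event, which also labels the notify.
; The sound comes from an audio bank the mesh owner supplies through I_FoleyAudioBankInterface, with volume and pitch multipliers applied.
; Run events also require the owner to allow footstep sounds.
; In the animation editor preview, it uses a default bank while the mesh is playing.
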(fn ReceivedNotify
  (params (MeshComp :type Skeletal%20Mesh%20Component%20Object%20Reference) (Animation :type Anim%20Sequence%20Base%20Object%20Reference) (EventReference :type Anim%20Notify%20Event%20Reference%20Structure%20%28by%20ref%29))
  (LocalVariables|SetMeshComponent MeshComp)
  (Utilities|IsValid (.Bank (CallFunction|GetAudioBank (LocalVariables|GetMeshComponent)))
    (:Is%20Valid
      (if (.CanPlaySound (CallFunction|GetAudioBank (LocalVariables|GetMeshComponent)))
        (Audio|PlaySoundatLocation (.Sound (Default|GetSoundfromFoleyEvent (.Bank (CallFunction|GetAudioBank (LocalVariables|GetMeshComponent))) (Variables|Default|GetEvent))) (Transformation|GetWorldLocation (LocalVariables|GetMeshComponent)) "0, 0, 0" (Variables|Default|GetVolumeMultiplier) (Variables|Default|GetPitchMultiplier) 0.0 0 0 0 0)
        (return true)))
    (:Is%20Not%20Valid
      (return false))))

(fn GetNotifyName
  (return (Utilities|String|ToString(Text) (Utilities|Text|FormatText "FoleyEvent: {Type}" (.RightS (Utilities|String|Split (GameplayTags|GetDebugStringfromGameplayTag (Variables|Default|GetEvent)) "." "IgnoreCase" "FromEnd"))))))

(fn GetAudioBank
  (params (MeshComponent :type Skeletal%20Mesh%20Component%20Object%20Reference))
  (bind _returnvalue (Components|GetOwner MeshComponent))
  (Utilities|Casting|CastToAnimationEditorPreviewActor _returnvalue
    (:then
      (if (Audio|Components|Audio|IsPlaying MeshComponent)
        (return (Variables|Default|GetDefaultBank) true)))
    (:CastFailed
      (if (Utilities|DoesObjectImplementInterface _returnvalue "/Game/Core/Audio/Foley/I_FoleyAudioBankInterface.I_FoleyAudioBankInterface_C")
        (bind _foleyaudiobank (Class|IFoleyAudioBankInterface|GetFoleyAudioBank(Message) _returnvalue))
        (if (GameplayTags|HasTag (GameplayTags|MakeLiteralGameplayTagContainer "(GameplayTags=((TagName=\"Foley.Event.Run\"),(TagName=\"Foley.Event.Scuff\"),(TagName=\"Foley.Event.Walk\"),(TagName=\"Foley.Event.RunBackwds\"),(TagName=\"Foley.Event.RunStrafe\"),(TagName=\"Foley.Event.WalkBackwds\"),(TagName=\"Foley.Event.ScuffPivot\"),(TagName=\"Foley.Event.Jump\"),(TagName=\"Foley.Event.Land\")))") (Variables|Default|GetEvent))
          (bind _returnvalue_2 (Class|IFoleyAudioBankInterface|CanPlayFootstepSounds(Message) _returnvalue))
          (return _foleyaudiobank _returnvalue_2)
          (else
            (return _foleyaudiobank true)))))))